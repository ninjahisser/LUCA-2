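; Player character that can be painted on with the mouse, with look rotation and wheel zoom on a spring arm.
; While left mouse is held, Tick traces under the cursor and paints wherever it hits the character itself.
; Each paint step captures the mesh with a temporary unwrap material, then draws a position/normal-driven material into the CRT_PaintMask render target.
; The mask clears on BeginPlay or a debug key, and painting still emits debug prints and arrows.
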(event EventBeginPlay
  (bind _returnvalue (Game|GetPlayerController 0))
  (Variables|/Script/Engine.PlayerController|SetbShowMouseCursor _returnvalue true)
  (Pawn|SetControlRotation _returnvalue (Math|Rotator|MakeRotator 0.0 0.0 1.8e+02))
  (Rendering|ClearRenderTarget2D "/Game/LEGODRAWIT/PaintSystem/CRT_PaintMask.CRT_PaintMask"))

(event EventTick
  (params (DeltaSeconds :type Float%20%28single-precision%29))
  (bind _returnvalue (Game|GetPlayerController 0))
  (bind (_worldlocation _worlddirection _returnvalue_2) (Game|Player|ConvertMouseLocationToWorldSpace _returnvalue))
  (if (Variables|Default|GetDrawing)
    (if _returnvalue_2
      (bind (_outhit _returnvalue_3) (Collision|LineTraceByChannel _worldlocation (+ _worldlocation (* _worlddirection 10000)) "TraceTypeQuery1" false 0 "None" false))
      (if _returnvalue_3
        (if (== (.HitActor (Collision|BreakHitResult _outhit)) self)
          (CallFunction|Paint (.ImpactPoint (Collision|BreakHitResult _outhit)) (.ImpactNormal (Collision|BreakHitResult _outhit))))))))

(event Input|MouseEvents|MouseWheelAxis
  (params (AxisValue :type Float%20%28single-precision%29))
  (CallFunction|Zoom (* AxisValue 5.0)))

(event Input|KeyboardEvents|DebugKeyC
  (params (Key :type Key%20Structure :default "None") (ActionValue :type Input%20Action%20Value%20Structure))
  (:Pressed
    (CallFunction|ClearPaint)))

(event Input|MouseEvents|LeftMouseButton
  (params (Key :type Key%20Structure :default "None"))
  (:Pressed
    (Variables|Default|SetDrawing true))
  (:Released
    (Variables|Default|SetDrawing false)))

(event Input|MouseEvents|Mouse2D
  (params (AxisValue :type Vector :default "0, 0, 0"))
  (bind (_x _y) (Math|Vector|BreakVector AxisValue))
  (if (not (Variables|Default|GetDrawing))
    (Pawn|Input|AddControllerYawInput _x)
    (Pawn|Input|AddControllerPitchInput (* _y -1.0))))

(fn ConstructionScript)

(fn Zoom
  (params (Zoom :type Float%20%28double-precision%29))
  (bind _springarm (Variables|Default|GetSpringArm))
  (Variables|/Script/Engine.SpringArmComponent|SetTargetArmLength _springarm (Math|Float|Clamp(Float) (- (Variables|/Script/Engine.SpringArmComponent|GetTargetArmLength _springarm) Zoom) (Variables|Default|GetZoom%20Min) (Variables|Default|GetZoom%20Max))))

(fn Unwrap
  (bind _mesh (Variables|Character|GetMesh))
  (bind _unwrapcapturecomponent (Variables|Default|GetUnwrapCaptureComponent))
  (Transformation|SetWorldRotation _unwrapcapturecomponent "-90.000000,-90.000000,0.000000" false false)
  (Rendering|SceneCapture|ShowOnlyComponent _unwrapcapturecomponent (Variables|Character|GetMesh))
  (bind _output_get (LocalVariables|SetOriginalMaterials (Rendering|Material|GetMaterials _mesh)))
  (for (_ _array_index) _output_get
    (Rendering|Material|SetMaterial _mesh _array_index "/Game/LEGODRAWIT/PaintSystem/M_Unwrap.M_Unwrap"))
  (Rendering|SceneCapture|CaptureScene (Variables|Default|GetUnwrapCaptureComponent) :!class /Script/Engine.SceneCaptureComponent2D)
  (for (_array_element _array_index_2) (LocalVariables|GetOriginalMaterials)
    (Rendering|Material|SetMaterial _mesh _array_index_2 _array_element)))

(fn Paint
  (params (Position :type Vector) (Normal :type Vector))
  (Development|PrintString (Utilities|String|ToString(Vector) Position))
  (Rendering|Debug|DrawDebugArrow Position (+ Position (* Normal 50)) 1.0 "(R=1.000000,G=1.000000,B=1.000000,A=1.000000)" 0.0 1.0)
  (CallFunction|Unwrap)
  (bind _returnvalue (Rendering|Material|CreateDynamicMaterialInstance "/Game/LEGODRAWIT/PaintSystem/M_PaintTexture.M_PaintTexture" "None" "None" :!class /Script/Engine.KismetMaterialLibrary))
  (Rendering|Material|SetVectorParameterValue _returnvalue "Position" (Math|Conversions|ToLinearColor(Vector) Position) :!class /Script/Engine.MaterialInstanceDynamic)
  (Rendering|Material|SetVectorParameterValue _returnvalue "Normal" (Math|Conversions|ToLinearColor(Vector) Normal) :!class /Script/Engine.MaterialInstanceDynamic)
  (Rendering|DrawMaterialtoRenderTarget "/Game/LEGODRAWIT/PaintSystem/CRT_PaintMask.CRT_PaintMask" _returnvalue))

(fn ClearPaint
  (Rendering|ClearRenderTarget2D "/Game/LEGODRAWIT/PaintSystem/CRT_PaintMask.CRT_PaintMask"))